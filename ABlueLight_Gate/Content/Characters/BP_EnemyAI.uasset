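; Enemy character that chases the player and explodes when caught in a visible light spot.
; PawnSensing sets a seen flag, never cleared here, and starts AIMoveTo toward the player unless dead.
; A Delay-throttled Tick polls capsule overlaps about every second, debug-printing visibility and looking for visible components tagged LightSpotTrigger.
; A match triggers death after a short delay, spawning an explosion before destroying the actor.
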(event OnSeePawn(PawnSensing)
  (params (Pawn :type Pawn%20Object%20Reference))
  (Variables|Default|SetisSeeingPlayer true)
  (if (not (Variables|Default|GetIsDead))
    (CallFunction|FollowPlayer)))

(event Custom|FollowPlayer
  (if (Variables|Default|GetisSeeingPlayer)
    (AI|AIMoveTo self "0.000000,0.000000,0.000000" (Game|GetPlayerCharacter 0) 5.0 false)))

(event Custom|Die
  (Variables|Default|SetIsDead true)
  (Effects|SpawnEmitteratLocation "/Game/StarterContent/Particles/P_Explosion.P_Explosion" (Transformation|GetWorldLocation (Variables|Collision|GetCapsuleComponent)))
  (Utilities|FlowControl|Delay 0.5)
  (Actor|DestroyActor))

(event EventBeginPlay)

(event Collision|EventActorBeginOverlap
  (params (OtherActor :type Actor%20Object%20Reference)))

(event EventTick
  (params (DeltaSeconds :type Float%20%28single-precision%29))
  (Utilities|FlowControl|Delay 1.0)
  (for _array_element (Class|PrimitiveComponent|GetOverlappingComponents (Variables|Collision|GetCapsuleComponent))
    (Development|PrintString (Utilities|String|ToString(Boolean) (Rendering|IsVisible _array_element)))
    (for _array_element_2 (Variables|/Script/Engine.ActorComponent|GetComponentTags _array_element)
      (if (and (== _array_element_2 "LightSpotTrigger") (Rendering|IsVisible _array_element))
        (Utilities|FlowControl|Delay 1.0)
        (CallFunction|Die)))))

(fn ConstructionScript)