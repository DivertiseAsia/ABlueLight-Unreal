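; Game instance that handles save slots, menu and loading-screen widgets, and background music.
; Events open the save slot and new game windows and delete saves.
; LoadGame reads the slot's save data, shows the loading screen and opens the last saved level, falling back to Stage-1 when none is recorded.
; PlayBGM creates and stores a 2D sound, but its stop-previous-track step is disconnected, so it never stops music already playing.
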(event Custom|RemoveLoadingScreen
  ;[1 1 1] Loading Screen
  (bind _loadingscreen (Variables|Default|GetLoadingScreen)
    (:then
      (Widget|RemovefromParent _loadingscreen))
    (:else)))

(event Custom|CreateLoadingScreen
  ;[1 1 1] Loading Screen
  (bind _scoreswidget (Variables|Default|GetScoresWidget)
    (:then
      (Widget|RemovefromParent _scoreswidget))
    (:else
      _))
  (bind _returnvalue (UserInterface|CreateWidget "/Game/Blueprints/Game/UI/WBP_LoadingScreen.WBP_LoadingScreen_C" (Game|GetPlayerController 0)))
  (bind _output_get (Variables|Default|SetLoadingScreen _returnvalue))
  (UserInterface|Viewport|AddtoViewport _output_get 0))

(event Custom|NewGame
  (params (GameSlot :type String))
  ;[1 1 1] Main Screen Commands
  (bind _newgamewindow (Variables|Default|GetNewGameWindow)
    (:then
      (Widget|RemovefromParent _newgamewindow))
    (:else
      _))
  (bind _returnvalue (UserInterface|CreateWidget "/Game/Blueprints/Game/UI/WBP_NewGame.WBP_NewGame_C" (Game|GetPlayerController 0) GameSlot))
  (bind _output_get (Variables|Default|SetNewGameWindow _returnvalue))
  (UserInterface|Viewport|AddtoViewport _output_get 0))

(event Custom|ShowMainScreenMenu
  ;[1 1 1] Main Screen Commands
  (bind _mainscreenmenu (Variables|Default|GetMainScreenMenu)
    (:then
      (Widget|RemovefromParent _mainscreenmenu))
    (:else
      _))
  (bind _returnvalue (UserInterface|CreateWidget "/Game/Blueprints/Game/UI/WBP_SaveSlotMenu.WBP_SaveSlotMenu_C" (Game|GetPlayerController 0)))
  (bind _output_get (Variables|Default|SetSaveSlotMenu _returnvalue))
  (UserInterface|Viewport|AddtoViewport _output_get 0))

(event Custom|LoadGame
  (params (SaveGameToLoad :type String))
  ;[1 1 1] Main Screen Commands
  (Variables|Default|SetCurrentSaveSlot SaveGameToLoad)
  (bind _returnvalue (SaveGame|DoesSaveGameExist SaveGameToLoad))
  (if _returnvalue
    (bind _returnvalue_2 (SaveGame|LoadGamefromSlot SaveGameToLoad))
    (bind _asbp_new_save_game (Utilities|Casting|CastToBP_NewSaveGame _returnvalue_2))
    (CallFunction|CreateLoadingScreen)
    (Variables|Default|SetSaveData (Variables|/Game/Blueprints/Game/BP_NewSaveGame.BP_NewSaveGame_C|GetSaveData _asbp_new_save_game))
    (Development|PrintString (.LastLevelSavedAt (Utilities|Struct|BreakS_SaveData (Variables|Default|GetSaveData))))
    (if (Utilities|Enum|NotEqual(Enum) (.LastLevelSavedAt (Utilities|Struct|BreakS_SaveData (Variables|Default|GetSaveData))) "")
      (Game|OpenLevel(byName) (Utilities|String|StringToName (.LastLevelSavedAt (Utilities|Struct|BreakS_SaveData (Variables|Default|GetSaveData)))))
      (else
        ;;[1 1 1] No Level Found
        (Game|OpenLevel(byName) "Stage-1")))
    (else
      (Development|PrintString (Utilities|String|ToString(Text) (Utilities|Text|FormatText "Failed to load save {save}" SaveGameToLoad))))))

(event Custom|DeleteGame
  (params (TargetSaveGame :type String))
  ;[1 1 1] Main Screen Commands
  (bind _returnvalue (SaveGame|DoesSaveGameExist TargetSaveGame))
  (if _returnvalue
    (SaveGame|DeleteGameinSlot TargetSaveGame)))

(fn StopBGM
  (bind _bgminstance (Variables|Default|GetBGMInstance))
  (Utilities|IsValid _bgminstance
    (:Is%20Valid
      (Audio|Components|Audio|FadeOut _bgminstance 0.0 0.0 "Linear" :!class /Script/Engine.AudioComponent))))

(fn PlayBGM
  (params (Sound :type Sound%20Base%20Object%20Reference) (VolumeMultiplier :type Float%20%28single-precision%29) (bPersistAcrossLevelTransition :type Boolean))
  (bind _returnvalue (Audio|CreateSound2D Sound VolumeMultiplier 1.0 0.0 0 bPersistAcrossLevelTransition false))
  (bind _output_get (Variables|Default|SetBGMInstance _returnvalue))
  (Audio|Components|Audio|Play _output_get 0.0))

(fn PlayTutorialBGM
  (CallFunction|PlayBGM "/Game/Audio/BackgroundMusic/BGMCue.BGMCue" 0.25 false))