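; BP_Fire_Handle is a fire prop whose flame and point light color follow a soul light state: off, normal, blue or violet.
; UpdateFireType swaps the Niagara flame asset, recolors the light and restores the default scale.
; Off only scales the flame to zero, leaving the light untouched.
; The update runs on construction, on BeginPlay and whenever SetFireTypeNumber changes the state.
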(event Custom|SetFireTypeNumber
  (params (CurrentSoulLight :type SoulLight%20Enum :default "NewEnumerator3"))
  (Variables|Default|SetCurrentSoulLight CurrentSoulLight)
  (CallFunction|UpdateFireType))

(event Custom|UpdateFireType
  (bind _pointlight (Variables|Default|GetPointLight))
  (bind _n_normalflame_em_system (Variables|Default|GetN_NormalFlame_EM_System))
  (switch Utilities|FlowControl|Switch|SwitchonSoulLight (Variables|Default|GetCurrentSoulLight)
    (:NewEnumerator3
      (Transformation|SetWorldScale3D _n_normalflame_em_system "0, 0, 0"))
    (:NewEnumerator0
      (Class|NiagaraComponent|SetAsset _n_normalflame_em_system "/Game/ThirdPerson/VFX/N_NormalFlame_EM_System.N_NormalFlame_EM_System" true)
      (Rendering|Components|Light|SetLightColor _pointlight "(R=1.000000,G=0.174217,B=0.134413,A=1.000000)" true)
      (Transformation|SetWorldScale3D _n_normalflame_em_system (Math|Conversions|ToVector(Float) (Variables|Default|GetDefaultScale)) :!label _label))
    (:NewEnumerator1
      (Class|NiagaraComponent|SetAsset _n_normalflame_em_system "/Game/ThirdPerson/VFX/N_BlueFlameTorch_EM_System.N_BlueFlameTorch_EM_System" true)
      (Rendering|Components|Light|SetLightColor _pointlight "(R=0.063010,G=0.854993,B=0.854993,A=1.000000)" true)
      (goto _label))
    (:NewEnumerator2
      (Class|NiagaraComponent|SetAsset _n_normalflame_em_system "/Game/ThirdPerson/VFX/N_VioletFlame_EM_System.N_VioletFlame_EM_System" true)
      (Rendering|Components|Light|SetLightColor _pointlight "(R=0.676728,G=0.000000,B=0.958333,A=1.000000)" true)
      (goto _label))))

(event EventBeginPlay
  (CallFunction|UpdateFireType))

(fn ConstructionScript
  (CallFunction|UpdateFireType))