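; Child fire Blueprint that adds a visible cooldown timer to an interactable soul light.
; Tick watches the light area's visibility through a DoOnce that re-arms while lit, so each switch-off triggers one countdown.
; A delayed loop updates the timer text every second, then clears it.
; Interact toggles the soul light, except during a countdown or when a lit fire is flagged as unable to turn off.
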(event Custom|Countdown
  (Variables|Default|SetCounting true)
  (Rendering|ToggleVisibility (Variables|Default|GetTextRender) true)
  (bind _index (Utilities|ForLoopwithDelay 1 (Variables|Default|GetTimer) 1.0)
    (:Loop%20Body
      (Rendering|Components|TextRender|SetText (Variables|Default|GetTextTimer) (Utilities|Text|ToText(Integer) (- (Variables|Default|GetTimer) _index))))
    (:Completed
      (Variables|Default|SetCounting false)
      (Rendering|Components|TextRender|SetText (Variables|Default|GetTextTimer) (Class|KismetTextLibrary|GetEmptyText))
      (Rendering|ToggleVisibility (Variables|Default|GetTextRender) true))))

(event EventBeginPlay
  (|CallParentFunction))

(event Collision|EventActorBeginOverlap
  (params (OtherActor :type Actor%20Object%20Reference)))

(event EventTick
  (params (DeltaSeconds :type Float%20%28single-precision%29))
  (if (Rendering|IsVisible (Variables|Default|Getvfx_light_area))
    (goto _label Reset)
    (else
      (Utilities|FlowControl|DoOnce true :!label _label
        (:Completed
          (CallFunction|Countdown))))))

(fn ConstructionScript
  (|CallParentFunction))

(fn Interact
  (params (Interactor :type Character%20Object%20Reference))
  (if (not (and (Rendering|IsVisible (Variables|Default|Getvfx_light_area)) (Variables|Default|GetCanNotTurnOff)))
    (if (not (Variables|Default|GetCounting))
      (CallFunction|ToggleSoulLight)
      (return true))))