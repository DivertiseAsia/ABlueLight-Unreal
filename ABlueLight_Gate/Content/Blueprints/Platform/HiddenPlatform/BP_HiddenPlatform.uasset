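; BP_HiddenPlatform is a platform whose PlatformPlane component slides along the Z axis between a shown and a hidden position.
; BeginPlay caches the plane's initial relative location as the shown position and binds handlers to the MoveToHide and MoveToShow dispatchers.
; Each handler uses MoveComponentTo: hiding offsets the plane by HideZAxis, and showing returns it to the cached location more slowly.
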(event Custom|MoveToHide_Event
  (bind _initpos (Variables|Default|GetInitPos))
  ;[1 1 1] Show/Hide Platform
  ;;[1 1 1] Move To Hide Platform
  (Components|MoveComponentTo (Variables|Default|GetPlatformPlane) (Math|Vector|MakeVector (.x _initpos) (.y _initpos) (+ (.z _initpos) (Variables|Default|GetHideZAxis))) "0, 0, 0" false false 1.0 false))

(event Custom|MoveToShow_Event
  ;[1 1 1] Show/Hide Platform
  ;;[1 1 1] Move To Show Platform
  (Components|MoveComponentTo (Variables|Default|GetPlatformPlane) (Variables|Default|GetInitPos) "0, 0, 0" false false 2.0 false))

(event EventBeginPlay
  (Variables|Default|SetInitPos (Variables|/Script/Engine.SceneComponent|GetRelativeLocation (Variables|Default|GetPlatformPlane)))
  (EventDispatchers|BindEventtoMovetoHide (delegate Custom|MoveToHide_Event))
  (EventDispatchers|BindEventtoMovetoShow (delegate Custom|MoveToShow_Event)))

(fn ConstructionScript)