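; Push-button actor that reveals a linked hidden platform, which it sends to its hidden state on BeginPlay.
; A trigger overlap with the third-person character enables input and opens a gate for the Interaction action.
; Pressing it plays a stone door sound and runs two timelines that lerp the button box in, then back out.
; The return timeline's updates call the platform's show event.
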(event OnComponentBeginOverlap(TriggerCollision)
  (params (OverlappedComponent :type Primitive%20Component%20Object%20Reference) (OtherActor :type Actor%20Object%20Reference) (OtherComp :type Primitive%20Component%20Object%20Reference) (OtherBodyIndex :type Integer) (bFromSweep :type Boolean) (SweepResult :type Hit%20Result%20Structure%20%28by%20ref%29))
  ;[1 1 1] Button Interaction (Push a Box)
  (Utilities|Casting|CastToBP_ThirdPersonCharacter OtherActor)
  (Input|EnableInput (Game|GetPlayerController 0))
  (Utilities|FlowControl|Gate true) ; enters at Open
)

(event OnComponentEndOverlap(TriggerCollision)
  (params (OverlappedComponent :type Primitive%20Component%20Object%20Reference) (OtherActor :type Actor%20Object%20Reference) (OtherComp :type Primitive%20Component%20Object%20Reference) (OtherBodyIndex :type Integer))
  ;[1 1 1] Button Interaction (Push a Box)
  (Utilities|Casting|CastToBP_ThirdPersonCharacter OtherActor)
  (Input|DisableInput (Game|GetPlayerController 0))
  (Utilities|FlowControl|Gate true) ; enters at Close
)

(event EventBeginPlay
  (bind _triggerobject (Variables|Default|GetTriggerObject))
  (bind _returnvalue (Transformation|GetRelativeTransform _triggerobject))
  (Variables|Default|SetOutPos (Math|Transform|MakeTransform (.location _returnvalue) (.rotation _returnvalue) (.scale _returnvalue)))
  (Variables|Default|SetInPos (Math|Transform|MakeTransform (/ (.location _returnvalue) "0,-100.000000,0") (.rotation _returnvalue) (.scale _returnvalue)))
  (Default|MovetoHideEvent (Variables|Default|GetHiddenPlatform)))

(event Input|ActionEvents|InputActionInteraction
  (params (Key :type Key%20Structure))
  ;[1 1 1] Button Interaction (Push a Box)
  (:Pressed
    (Utilities|FlowControl|Gate true
      (:Exit
        ;[1 1 1] Box Animation
        (|Animation_BoxInOut
          (:Out
            ;[1 1 1] Show Hidden Platform
            (Default|MovetoShowEvent (Variables|Default|GetHiddenPlatform))))))))

(fn ConstructionScript)