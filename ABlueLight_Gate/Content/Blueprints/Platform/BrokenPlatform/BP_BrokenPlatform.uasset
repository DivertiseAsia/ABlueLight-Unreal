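; BP_BrokenPlatform is a platform that breaks and falls after the third-person character steps on it, either when its countdown expires or shortly after they leave.
; Box overlaps set a state that Tick reads, with a Delay pacing the countdown in seconds.
; Near the end it starts a camera shake and earthquake sound once.
; Breaking stops the sound, moves the mesh far downward and destroys the actor.
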(event OnComponentBeginOverlap(BoxCollision)
  (params (OverlappedComponent :type Primitive%20Component%20Object%20Reference) (OtherActor :type Actor%20Object%20Reference) (OtherComp :type Primitive%20Component%20Object%20Reference) (OtherBodyIndex :type Integer) (bFromSweep :type Boolean) (SweepResult :type Hit%20Result%20Structure%20%28by%20ref%29))
  ;[1 1 1] Player Step On
  (Utilities|Casting|CastToBP_ThirdPersonCharacter OtherActor)
  (Variables|Default|SetPlatformState "NewEnumerator1"))

(event OnComponentEndOverlap(BoxCollision)
  (params (OverlappedComponent :type Primitive%20Component%20Object%20Reference) (OtherActor :type Actor%20Object%20Reference) (OtherComp :type Primitive%20Component%20Object%20Reference) (OtherBodyIndex :type Integer))
  ;[1 1 1] Player Step Out
  (Utilities|Casting|CastToBP_ThirdPersonCharacter OtherActor)
  (CallFunction|StopCameraShake)
  (Utilities|FlowControl|Delay 0.5)
  (Variables|Default|SetPlatformState "NewEnumerator2"))

(event EventBeginPlay
  (Variables|Default|SetBrokenCount (Variables|Default|GetBrokenInSec)))

(event EventTick
  (params (DeltaSeconds :type Float%20%28single-precision%29))
  (switch Utilities|FlowControl|Switch|SwitchonENUM_BrokenPlatformState (Variables|Default|GetPlatformState)
    (:NewEnumerator1
      (|PlayerStepOnLogic))
    (:NewEnumerator2
      (Utilities|FlowControl|DoOnce false
        (:Completed
          (|BrokePlatformLogic))))))

(fn ConstructionScript)

(fn ShakeCamera
  (bind _returnvalue (Class|MatineeCameraShake|StartMatineeCameraShake (Game|GetPlayerCameraManager 0) "/Game/Blueprints/Platform/BrokenPlatform/BP_BrokenPlatformCameraShake.BP_BrokenPlatformCameraShake_C" 1.0 "CameraLocal" "0, 0, 0"))
  (Variables|Default|SetCameraShakeRef _returnvalue))

(fn StopCameraShake
  (bind _camerashakeref (Variables|Default|GetCameraShakeRef))
  (Utilities|IsValid _camerashakeref
    (:Is%20Valid
      (CameraShakes|StopCameraShake (Game|GetPlayerCameraManager 0) _camerashakeref true))))