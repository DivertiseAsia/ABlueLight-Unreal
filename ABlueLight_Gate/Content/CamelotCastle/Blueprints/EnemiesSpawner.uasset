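; EnemiesSpawner is an actor that keeps spawning BP_EnemyAI enemies at its own location while few of them exist in the level.
; Tick runs through a Delay set by the Delay variable, then calls the Spawner event.
; Spawner counts all BP_EnemyAI actors and, if fewer than two exist, waits briefly before spawning another with SpawnAIFromClass.
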(event Custom|Spawner
  (bind _outactors (Actor|GetAllActorsOfClass "/Game/Characters/BP_EnemyAI.BP_EnemyAI_C"))
  (if (< (Utilities|Array|Length _outactors) 2)
    (Utilities|FlowControl|Delay 2.0)
    (AI|SpawnAIFromClass "/Game/Characters/BP_EnemyAI.BP_EnemyAI_C" 0 (Transformation|GetActorLocation self) "0, 0, 0" false 0)))

(event EventBeginPlay)

(event EventTick
  (params (DeltaSeconds :type Float%20%28single-precision%29))
  (Utilities|FlowControl|Delay (Variables|Default|Getdelay))
  (CallFunction|Spawner))

(fn ConstructionScript)