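; Game mode that saves and restores the third-person character's transform and health through a single save slot.
; On BeginPlay it applies the saved data to the player, or creates a fresh save file if none exists.
; SaveGame overwrites the slot with current values, while LoadGame just restarts the level so BeginPlay reapplies them.
; RestartLevel deletes the save before restarting, giving a clean start.
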(event Custom|SaveGame
  (bind _returnvalue (Game|GetPlayerCharacter 0))
  (bind _asbp_third_person_character (Utilities|Casting|CastToBP_ThirdPersonCharacter _returnvalue))
  ;[1 1 1] Save Game
  (bind _returnvalue_2 (SaveGame|LoadGamefromSlot "Save"))
  (bind _asbp_save_game (Utilities|Casting|CastToBP_SaveGame _returnvalue_2))
  (Variables|/Game/SaveGames/BP_SaveGame.BP_SaveGame_C|SetLocation _asbp_save_game (Transformation|GetActorTransform _asbp_third_person_character))
  (Variables|/Game/SaveGames/BP_SaveGame.BP_SaveGame_C|SetHealth _asbp_save_game (Variables|/Game/ThirdPerson/Blueprints/BP_ThirdPersonCharacter.BP_ThirdPersonCharacter_C|GetHealth _asbp_third_person_character))
  (SaveGame|SaveGametoSlot _asbp_save_game "Save"))

(event Custom|LoadGame
  ;[1 1 1] Load Game
  (Development|ExecuteConsoleCommand "RestartLevel" 0))

(event Custom|RestartLevel
  ;[1 1 1] Delete Save + Restart
  (SaveGame|DeleteGameinSlot "Save")
  (Development|ExecuteConsoleCommand "RestartLevel" 0))

(event EventBeginPlay
  (bind _returnvalue (SaveGame|DoesSaveGameExist "Save"))
  (if _returnvalue
    ;[1 1 1] Load Game
    (bind _returnvalue_2 (SaveGame|LoadGamefromSlot "Save"))
    (bind _asbp_save_game (Utilities|Casting|CastToBP_SaveGame _returnvalue_2))
    (bind _asbp_third_person_character (Utilities|Casting|CastToBP_ThirdPersonCharacter (Game|GetPlayerCharacter 0)))
    (Transformation|SetWorldTransform (Variables|/Script/Engine.Actor|GetRootComponent _asbp_third_person_character) (Variables|/Game/SaveGames/BP_SaveGame.BP_SaveGame_C|GetLocation _asbp_save_game) false false)
    (Variables|/Game/ThirdPerson/Blueprints/BP_ThirdPersonCharacter.BP_ThirdPersonCharacter_C|SetHealth _asbp_third_person_character (Variables|/Game/SaveGames/BP_SaveGame.BP_SaveGame_C|GetHealth _asbp_save_game))
    (else
      ;[1 1 1] Create Save File
      (bind _returnvalue_3 (SaveGame|CreateSaveGameObject "/Game/SaveGames/BP_SaveGame.BP_SaveGame_C"))
      (SaveGame|SaveGametoSlot _returnvalue_3 "Save"))))

(fn ConstructionScript)