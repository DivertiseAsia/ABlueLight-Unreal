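; DoorController is a puzzle gate that opens a door once every fire base in its LightTowers array is lit.
; Tick feeds a one-second Delay, acting as a periodic check that each BP_FireBase_Child's VfxLightArea is visible.
; When all are, the DoorActivation timeline animates the Door static mesh actor's relative Z.
; The controller destroys itself when the timeline finishes.
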(event EventBeginPlay)

(event Collision|EventActorBeginOverlap
  (params (OtherActor :type Actor%20Object%20Reference)))

(event EventTick
  (params (DeltaSeconds :type Float%20%28single-precision%29))
  (Utilities|FlowControl|Delay 1.0)
  (Variables|Default|SetClearCondition true)
  (for _array_element (Variables|Default|GetLightTowers)
    (bind _asbp_fire_base_child (Utilities|Casting|CastToBP_FireBase_Child _array_element))
    (if (not (Rendering|IsVisible (Variables|/Game/ThirdPerson/Blueprints/Fire/BP_FireBase.BP_FireBase_C|Getvfx_light_area _asbp_fire_base_child)))
      (Variables|Default|SetClearCondition false)))
  (if (Variables|Default|GetClearCondition)
    (bind _asstatic_mesh_actor (Utilities|Casting|CastToStaticMeshActor (Variables|Default|GetDoor)))
    (bind _doorposition (Timeline|DoorActivation Play)
      (:Update
        (Transformation|SetRelativeLocation (Variables|/Script/Engine.StaticMeshActor|GetStaticMeshComponent _asstatic_mesh_actor) (Math|Vector|MakeVector (.x (Variables|/Script/Engine.SceneComponent|GetRelativeLocation (Variables|/Script/Engine.StaticMeshActor|GetStaticMeshComponent _asstatic_mesh_actor))) (.y (Variables|/Script/Engine.SceneComponent|GetRelativeLocation (Variables|/Script/Engine.StaticMeshActor|GetStaticMeshComponent _asstatic_mesh_actor))) _doorposition) false false))
      (:Finished
        (Actor|DestroyActor)))))

(fn ConstructionScript)