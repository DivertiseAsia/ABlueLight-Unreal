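; Stage progression controller that opens doors based on enemy and light tower state.
; A delayed Tick poll opens the first door once the first enemy is gone, and sets the spawner's condition flag when every tower's light effect is visible.
; With that flag set, it opens the last door when the spawner's MaximumAI runs out, printing the remaining enemy count.
; A shared timeline animates each door's Z position.
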(event Custom|ActivateDoor
  (params (Door :type Actor%20Object%20Reference))
  ;[1 1 1] Activate Door
  (bind _asstatic_mesh_actor (Utilities|Casting|CastToStaticMeshActor Door))
  (bind _doorposition (Timeline|FirstDoorActivation Play)
    (:Update
      (Transformation|SetRelativeLocation (Variables|/Script/Engine.StaticMeshActor|GetStaticMeshComponent _asstatic_mesh_actor) (Math|Vector|MakeVector (.x (Variables|/Script/Engine.SceneComponent|GetRelativeLocation (Variables|/Script/Engine.StaticMeshActor|GetStaticMeshComponent _asstatic_mesh_actor))) (.y (Variables|/Script/Engine.SceneComponent|GetRelativeLocation (Variables|/Script/Engine.StaticMeshActor|GetStaticMeshComponent _asstatic_mesh_actor))) _doorposition) false false))))

(event Custom|CheckLightTowers
  (Variables|Default|SetClearedCondition true)
  (for _array_element (Variables|Default|GetLightTowers)
    (if (not (Rendering|IsVisible (Variables|/Game/Blueprints/Fire/BP_FireBase.BP_FireBase_C|Getvfx_light_area _array_element)))
      (Variables|Default|SetClearedCondition false)))
  (if (Variables|Default|GetClearedCondition)
    (Variables|/Game/CamelotCastle/Blueprints/EnemiesSpawner.EnemiesSpawner_C|SetOtherCondition (Variables|Default|GetEnemySpawner) true)))

(event EventBeginPlay)

(event Collision|EventActorBeginOverlap
  (params (OtherActor :type Actor%20Object%20Reference)))

(event EventTick
  (params (DeltaSeconds :type Float%20%28single-precision%29))
  (bind _enemyspawner (Variables|Default|GetEnemySpawner))
  (Utilities|FlowControl|Delay 1.0)
  (if (Variables|/Game/CamelotCastle/Blueprints/EnemiesSpawner.EnemiesSpawner_C|GetOtherCondition _enemyspawner)
    (if (<= (Variables|/Game/CamelotCastle/Blueprints/EnemiesSpawner.EnemiesSpawner_C|GetMaximumAI _enemyspawner) 0)
      (bind _outactors (Actor|GetAllActorsOfClass "/Game/Characters/BP_EnemyAI.BP_EnemyAI_C"))
      (Development|PrintString (Utilities|String|ToString(Integer) (Utilities|Array|Length _outactors)))
      (CallFunction|ActivateDoor (Variables|Default|GetLastDoor)))
    (else
      (CallFunction|CheckLightTowers)
      (if (not (Utilities|IsValid (Variables|Default|GetFirstEnemy)))
        (Utilities|FlowControl|DoOnce false
          (:Completed
            (CallFunction|ActivateDoor (Variables|Default|GetFirstDoor))))))))

(fn ConstructionScript)