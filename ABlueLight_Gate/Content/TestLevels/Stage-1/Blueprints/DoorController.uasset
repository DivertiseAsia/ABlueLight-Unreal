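; DoorController is a Stage-1 test level actor that opens a stone door once all linked light towers are lit.
; Tick runs through a one-second Delay, so it polls roughly every second whether each tower's VfxLightArea is visible.
; When all are, it plays the door sound and a timeline moves the door's Z position, then the controller destroys itself.
; On BeginPlay it also starts the tutorial music through GI_GameInstance.
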(event EventBeginPlay
  (bind _asgi_game_instance (Utilities|Casting|CastToGI_GameInstance (Game|GetGameInstance)))
  (Default|PlayTutorialBGM _asgi_game_instance)
  (Development|PrintString "PLAYED BGM"))

(event Collision|EventActorBeginOverlap
  (params (OtherActor :type Actor%20Object%20Reference)))

(event EventTick
  (params (DeltaSeconds :type Float%20%28single-precision%29))
  (bind _door (Variables|Default|GetDoor))
  (Utilities|FlowControl|Delay 1.0)
  (Variables|Default|SetClearCondition true)
  (for _array_element (Variables|Default|GetLightTowers)
    (bind _asbp_fire_base_child (Utilities|Casting|CastToBP_FireBase_Child _array_element))
    (if (not (Rendering|IsVisible (Variables|/Game/Blueprints/Fire/BP_FireBase.BP_FireBase_C|Getvfx_light_area _asbp_fire_base_child)))
      (Variables|Default|SetClearCondition false)))
  (if (Variables|Default|GetClearCondition)
    (bind _asstatic_mesh_actor (Utilities|Casting|CastToStaticMeshActor _door))
    (Audio|PlaySoundatLocation "/Game/Audio/SoundEffects/StoneDoorOpenCue.StoneDoorOpenCue" (Transformation|GetActorLocation _door) "0, 0, 0" 1.0 1.0 0.0 0 0 0 0)
    (bind _doorposition (Timeline|DoorActivation Play)
      (:Update
        (Transformation|SetRelativeLocation (Variables|/Script/Engine.StaticMeshActor|GetStaticMeshComponent _asstatic_mesh_actor) (Math|Vector|MakeVector (.x (Variables|/Script/Engine.SceneComponent|GetRelativeLocation (Variables|/Script/Engine.StaticMeshActor|GetStaticMeshComponent _asstatic_mesh_actor))) (.y (Variables|/Script/Engine.SceneComponent|GetRelativeLocation (Variables|/Script/Engine.StaticMeshActor|GetStaticMeshComponent _asstatic_mesh_actor))) _doorposition) false false))
      (:Finished
        (Actor|DestroyActor)))))

(fn ConstructionScript)